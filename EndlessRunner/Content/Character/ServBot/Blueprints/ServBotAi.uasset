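; ServBotAi is an AI ServBot that wanders between level TargetPoints and approaches other ServBots it sees.
; RandomMovePoints picks two random TargetPoints and a random walk speed, then MoveToTarget alternates between them via FlipFlop, re-rolling after each move ends.
; PawnSensing sets InRange, which blocks MoveToTarget, before casting to ServBotAi.
; Only a successful cast starts the approach, whose end clears the flag and resumes wandering after a short delay.
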(event `self.PawnSensing.OnSeePawn`
  (params (Pawn :type "Pawn Object Reference"))
  ;[1 1 1] Sense Pawn, move to
  (set `self.inRange?` true)
  (bind _asserv_bot_ai (cast `/Game/Character/ServBot/Blueprints/ServBotAi` Pawn))
  (`|AIMoveTo` self (0.0 0.0 0.0) _asserv_bot_ai
    (:`OnSuccess`
      _)
    (:`OnFail`
      _))
  (`KismetSystemLibrary.Delay` 0.2)
  (set `self.inRange?` false)
  (`self.MoveToTarget`))

(event `MoveToTarget`
  ;[1 1 1] move to target points
  (if (not (`self.inRange?`))
    (`/Engine/EditorBlueprintResources/StandardMacros.FlipFlop`
      (:`A`
        (`|AIMoveTo` self (0.0 0.0 0.0) (`self.targetpoint1`)
          (:`OnSuccess`
            _)
          (:`OnFail`
            _)))
      (:`B`
        (`|AIMoveTo` self (0.0 0.0 0.0) (`self.targetpoint2`)
          (:`OnSuccess`
            _)
          (:`OnFail`
            _))))
    (`self.RandomMovePoints`)))

(event `RandomMovePoints`
  ;[1 1 1] RandomMoveToPoint
  (bind _outactors (`GameplayStatics.GetAllActorsOfClass` "/Script/Engine.TargetPoint"))
  (`|ExecutionSequence`
    (:`then_0`
      (for (_ _array_index) _outactors
        (bind _output_get (set `self.maxTargetPoints` _array_index))))
    (:`then_1`
      (`|ExecutionSequence`
        (:`then_0`
          (set `self.Point1Index` (`KismetMathLibrary.RandomIntegerInRange` 0 _output_get))
          (set `CharacterMovementComponent.MaxWalkSpeed` (`KismetMathLibrary.Conv_IntToDouble` (`KismetMathLibrary.RandomIntegerInRange` 50 150)) (`self.CharacterMovement`)))
        (:`then_1`
          (set `self.Point2Index` (`KismetMathLibrary.RandomIntegerInRange` 0 _output_get)))))
    (:`then_2`
      (for (_array_element _array_index_2) _outactors
        (if (== (`self.Point1Index`) _array_index_2)
          (set `self.targetpoint1` _array_element))))
    (:`then_3`
      (for (_array_element_2 _array_index_3) _outactors
        (if (== (`self.Point2Index`) _array_index_3)
          (set `self.targetpoint2` _array_element_2))))
    (:`then_4`
      (`self.MoveToTarget`))))

(event `self.ReceiveBeginPlay`
  ;[1 1 1] Events
  (`self.RandomMovePoints`))

(fn `UserConstructionScript`)