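; DashGameMode_BP is the game mode for a dash-style runner level, starting background music and building the initial track of ruin tiles.
; The construction script seeds SpawnTransform from the root component's world transform.
; On BeginPlay it plays a 2D music cue and calls AddTile ten times.
; Each AddTile spawns a BP_RuinTile at SpawnTransform, then moves SpawnTransform to that tile's attach transform, chaining tiles end to end.
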(event `self.ReceiveBeginPlay`
  (bind _returnvalue (`GameplayStatics.CreateSound2D` "/Game/Audio/SoundTrack/Were_the_Bonnes__Cue.Were_the_Bonnes__Cue" 1.0 1.0 0.0 null))
  (`AudioComponent.Play` _returnvalue 0.0)
  (for _ (range 10)
    (`self.AddTile`)))

(fn `AddTile`
  (bind _returnvalue (`self.AddRuinTile` (`self.SpawnTransform`)))
  (bind _asbp_ruin_tile (cast `/Game/Blueprints/Tiles/BP_RuinTile` _returnvalue))
  (bind _attachpointtransform (`/Game/Blueprints/Tiles/BP_RuinTile.getAttachTransform` _asbp_ruin_tile))
  (set `self.SpawnTransform` _attachpointtransform))

(fn `UserConstructionScript`
  (set `self.SpawnTransform` (`SceneComponent.K2_GetComponentToWorld` (`self.DefaultSceneRoot`))))