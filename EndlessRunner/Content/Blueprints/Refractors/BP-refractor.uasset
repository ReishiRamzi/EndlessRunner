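; Collectible pickup for the endless runner that adds its Value to the runner's coins when the character overlaps its mesh.
; With the magnet active, a timeline pulls it toward player 0 via VInterpTo plus a track offset, then collects it after a short delay.
; Otherwise it collects immediately, and RemoveRefractor plays a sound, spawns an emitter and destroys the actor.
; MoveToRunner is an empty stub.
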(event `self.StaticMesh.OnComponentBeginOverlap`
  (params (OverlappedComponent :type "PrimitiveComponent Object Reference") (OtherActor :type "Actor Object Reference") (OtherComp :type "PrimitiveComponent Object Reference") (OtherBodyIndex :type Integer) (bFromSweep :type Boolean) (SweepResult :type "HitResult Structure (by ref)"))
  (bind _asendless_run_character (cast `/Game/Blueprints/EndlessRunCharacter` OtherActor))
  (if (`/Game/Blueprints/EndlessRunCharacter.isMagnetActive` _asendless_run_character)
    (bind (_direction _newtrack_0) (`Timeline|Timeline_0` :!via `PlayFromStart`)
      (:`Update`
        (`self.K2_SetActorLocation` (+ _newtrack_0 (`KismetMathLibrary.VInterpTo` (.location (`self.GetTransform`)) (`self.K2_GetActorLocation` (`GameplayStatics.GetPlayerCharacter` 0)) (`GameplayStatics.GetWorldDeltaSeconds`) 10.0)))
        (`KismetSystemLibrary.Delay` 0.2))))
  (`/Game/Blueprints/EndlessRunCharacter.addCoin` _asendless_run_character (`self.Value`))
  (`self.RemoveRefractor`))

(fn `MoveToRunner`)

(fn `RemoveRefractor`
  (bind _returnvalue (`self.K2_GetActorLocation`))
  (`GameplayStatics.PlaySoundAtLocation` "/Game/Audio/SFX/sfx-getzenny1.sfx-getzenny1" _returnvalue (struct) 1.0 1.0 0.0 null null null)
  (`GameplayStatics.SpawnEmitterAtLocation` null _returnvalue)
  (`self.K2_DestroyActor`))

(fn `UserConstructionScript`)