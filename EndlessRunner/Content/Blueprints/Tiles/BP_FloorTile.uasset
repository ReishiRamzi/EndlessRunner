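; BP_FloorTile is a floor segment for an endless runner, exposing an attach-point transform.
; Its construction script randomly scatters child-actor coins inside CoinArea, using a random switch per coin, and adds a blocker at one of three spawn points.
; When EndlessRunCharacter overlaps EndTrigger, the tile asks the game mode to add another tile, then destroys itself after a short delay.
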(event `self.endTrigger.OnComponentBeginOverlap`
  (params (OverlappedComponent :type "PrimitiveComponent Object Reference") (OtherActor :type "Actor Object Reference") (OtherComp :type "PrimitiveComponent Object Reference") (OtherBodyIndex :type Integer) (bFromSweep :type Boolean) (SweepResult :type "HitResult Structure (by ref)"))
  (cast `/Game/Blueprints/EndlessRunCharacter` OtherActor)
  (bind _asendless_run_game_mode (cast `/Game/Blueprints/endlessRunGameMode` (`GameplayStatics.GetGameMode`)))
  (`/Game/Blueprints/endlessRunGameMode.addFloorTile` _asendless_run_game_mode)
  (`KismetSystemLibrary.Delay` 2.0)
  (`self.K2_DestroyActor`))

(fn `getAttachTransform`
  (returns (attachPointTransform :type "Transform Structure"))
  (return (`SceneComponent.K2_GetComponentToWorld` (`self.attachPoint`))))

(fn `setSpawnPoints`
  (set `self.SpawnPoints` (`|MakeArray` (`SceneComponent.GetRelativeTransform` (`self.SpawnPoint_01`)) (`SceneComponent.GetRelativeTransform` (`self.SpawnPoint_02`)) (`SceneComponent.GetRelativeTransform` (`self.SpawnPoint_03`)))))

(fn `spawnBlocker`
  (bind _spawnpoints (`self.SpawnPoints`))
  (`AddComponent|NODE_AddChildActorComponent-0` :`RelativeTransform` (`|GetArrayItem` _spawnpoints (`KismetMathLibrary.RandomIntegerInRange` 0 (`KismetArrayLibrary.Array_LastIndex` _spawnpoints)))))

(fn `spawnCoins`
  (bind _coinarea (`self.coinArea`))
  (bind _returnvalue (`KismetMathLibrary.Conv_VectorToTransform` (`KismetMathLibrary.RandomPointInBoundingBox` (`SceneComponent.RelativeLocation` _coinarea) (`BoxComponent.BoxExtent` _coinarea))))
  (for _ (range (+ (`KismetMathLibrary.RandomIntegerInRange` 3 10) 1))
    (switch `int` (`KismetMathLibrary.RandomIntegerInRange` 0 3)
      (:`Default`
        (`AddComponent|NODE_AddChildActorComponent-5` :`RelativeTransform` _returnvalue :!label _label))
      (:`0`
        (goto _label))
      (:`1`
        (`AddComponent|NODE_AddChildActorComponent-6` :`RelativeTransform` _returnvalue))
      (:`2`
        (`AddComponent|NODE_AddChildActorComponent-7` :`RelativeTransform` _returnvalue))
      (:`3`
        (`AddComponent|NODE_AddChildActorComponent-8` :`RelativeTransform` _returnvalue)))))

(fn `UserConstructionScript`
  (`self.setSpawnPoints`)
  (`self.spawnCoins`)
  (`self.spawnBlocker`))