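; Endless-runner ruin track tile that asks DashGameState to add the next ruin tile at its SpawnAttachPoint when the runner overlaps TileEndTrigger.
; The construction script populates it with child actors, scattering random coins inside the CoinArea box.
; Player Zenny thresholds gate harder content: a blocker at one of three spawn points, then an occasional random pickup in the coin area.
; HitWall is an empty stub.
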(event `self.TileEndTrigger.OnComponentBeginOverlap`
  (params (OverlappedComponent :type "PrimitiveComponent Object Reference") (OtherActor :type "Actor Object Reference") (OtherComp :type "PrimitiveComponent Object Reference") (OtherBodyIndex :type Integer) (bFromSweep :type Boolean) (SweepResult :type "HitResult Structure (by ref)"))
  (cast `/Game/Blueprints/EndlessRunCharacter` OtherActor)
  (bind _asdash_game_state (cast `DashGameState` (`GameplayStatics.GetGameState`)))
  (`DashGameState.AddRuinTile` _asdash_game_state (`self.SpawnAttachPoint`)))

(fn `hitWall`
  (params (actor :type "Actor Object Reference") (hitNormal :type "Vector Structure")))

(fn `setSpawnPoints`
  (set `self.SpawnPoints` (`|MakeArray` (`SceneComponent.GetRelativeTransform` (`self.SpawnPoint_01`)) (`SceneComponent.GetRelativeTransform` (`self.SpawnPoint_02`)) (`SceneComponent.GetRelativeTransform` (`self.SpawnPoint_03`)))))

(fn `spawnBlocker`
  (bind _spawnpoints (`self.SpawnPoints`))
  (bind _asendless_run_character (cast `/Game/Blueprints/EndlessRunCharacter` (`GameplayStatics.GetPlayerCharacter` 0)))
  (if (> (`Servbot.Zenny` _asendless_run_character) 5000)
    (`AddComponent|NODE_AddChildActorComponent-0` :`RelativeTransform` (`|GetArrayItem` _spawnpoints (`KismetMathLibrary.RandomIntegerInRange` 0 (`KismetArrayLibrary.Array_LastIndex` _spawnpoints))))))

(fn `spawnCoins`
  (bind _coinarea (`self.coinArea`))
  (bind _returnvalue_location (`KismetMathLibrary.BreakTransform` (`SceneComponent.GetRelativeTransform` _coinarea)))
  (bind _returnvalue (`KismetMathLibrary.Conv_VectorToTransform` (`KismetMathLibrary.RandomPointInBoundingBox` _returnvalue_location (`BoxComponent.BoxExtent` _coinarea))))
  (for _ (range (+ (`KismetMathLibrary.RandomIntegerInRange` 3 7) 1))
    (switch `int` (`KismetMathLibrary.RandomIntegerInRange` 0 3)
      (:`Default`
        (`AddComponent|NODE_AddChildActorComponent-5` :`RelativeTransform` _returnvalue :!label _label))
      (:`0`
        (goto _label))
      (:`1`
        (`AddComponent|NODE_AddChildActorComponent-6` :`RelativeTransform` _returnvalue))
      (:`2`
        (`AddComponent|NODE_AddChildActorComponent-7` :`RelativeTransform` _returnvalue))
      (:`3`
        (`AddComponent|NODE_AddChildActorComponent-8` :`RelativeTransform` _returnvalue)))))

(fn `spawnPickup`
  (bind _coinarea (`self.coinArea`))
  (bind _returnvalue_location (`KismetMathLibrary.BreakTransform` (`SceneComponent.GetRelativeTransform` _coinarea)))
  (bind _asendless_run_character (cast `/Game/Blueprints/EndlessRunCharacter` (`GameplayStatics.GetPlayerCharacter` 0)))
  (if (> (`Servbot.Zenny` _asendless_run_character) 10000)
    (if (== (`KismetMathLibrary.RandomIntegerInRange` 0 5) 2)
      (`AddComponent|NODE_AddChildActorComponent-10` :`RelativeTransform` (`KismetMathLibrary.Conv_VectorToTransform` (`KismetMathLibrary.RandomPointInBoundingBox` _returnvalue_location (`BoxComponent.BoxExtent` _coinarea)))))))

(fn `UserConstructionScript`
  (`self.setSpawnPoints`)
  (`self.spawnCoins`)
  (`self.spawnBlocker`)
  (`self.spawnPickup`))