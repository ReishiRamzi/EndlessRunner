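; BP_RuinTile is a floor tile for an endless runner that fills itself with coins and an optional blocker.
; Construction scatters random child actors in CoinArea and adds a blocker at one of three spawn points once the player's TotalCoins passes a threshold.
; Crossing EndTrigger has the game mode add another tile, then destroys this one after a delay.
; Wall hits kill the runner when a dot-product test shows a head-on impact.
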(event `self.endTrigger.OnComponentBeginOverlap`
  (params (OverlappedComponent :type "PrimitiveComponent Object Reference") (OtherActor :type "Actor Object Reference") (OtherComp :type "PrimitiveComponent Object Reference") (OtherBodyIndex :type Integer) (bFromSweep :type Boolean) (SweepResult :type "HitResult Structure (by ref)"))
  (bind _asendless_run_character (cast `/Game/Blueprints/EndlessRunCharacter` OtherActor))
  (set `self.EndlessCharacter` _asendless_run_character)
  (bind _asendless_run_game_mode (cast `/Game/Blueprints/endlessRunGameMode` (`GameplayStatics.GetGameMode`)))
  (`/Game/Blueprints/endlessRunGameMode.addFloorTile` _asendless_run_game_mode)
  (`KismetSystemLibrary.Delay` 1.0)
  (`self.K2_DestroyActor`))

(event `self.Wall_R_01.OnComponentHit`
  (params (HitComponent :type "PrimitiveComponent Object Reference") (OtherActor :type "Actor Object Reference") (OtherComp :type "PrimitiveComponent Object Reference") (NormalImpulse :type "Vector Structure") (Hit :type "HitResult Structure (by ref)"))
  (`self.hitWall` OtherActor Hit_Normal))

(event `self.Wall_R_02.OnComponentHit`
  (params (HitComponent :type "PrimitiveComponent Object Reference") (OtherActor :type "Actor Object Reference") (OtherComp :type "PrimitiveComponent Object Reference") (NormalImpulse :type "Vector Structure") (Hit :type "HitResult Structure (by ref)"))
  (`self.hitWall` OtherActor Hit_Normal))

(event `self.Wall_L01.OnComponentHit`
  (params (HitComponent :type "PrimitiveComponent Object Reference") (OtherActor :type "Actor Object Reference") (OtherComp :type "PrimitiveComponent Object Reference") (NormalImpulse :type "Vector Structure") (Hit :type "HitResult Structure (by ref)"))
  (`self.hitWall` OtherActor Hit_Normal))

(event `self.Wall_L_02.OnComponentHit`
  (params (HitComponent :type "PrimitiveComponent Object Reference") (OtherActor :type "Actor Object Reference") (OtherComp :type "PrimitiveComponent Object Reference") (NormalImpulse :type "Vector Structure") (Hit :type "HitResult Structure (by ref)"))
  (`self.hitWall` OtherActor Hit_Normal))

(fn `getAttachTransform`
  (returns (attachPointTransform :type "Transform Structure"))
  (return (`SceneComponent.K2_GetComponentToWorld` (`self.attachPoint`))))

(fn `hitWall`
  (params (actor :type "Actor Object Reference") (hitNormal :type "Vector Structure"))
  (bind _asendless_run_character (cast `/Game/Blueprints/EndlessRunCharacter` actor))
  (bind _returnvalue (`KismetMathLibrary.Dot_VectorVector` hitNormal (`self.GetActorForwardVector` _asendless_run_character)))
  (if (or (`KismetMathLibrary.NearlyEqual_FloatFloat` _returnvalue -1.0 0.2) (`KismetMathLibrary.NearlyEqual_FloatFloat` _returnvalue 1.0 0.2))
    (`/Game/Blueprints/EndlessRunCharacter.death` _asendless_run_character)))

(fn `setSpawnPoints`
  (set `self.SpawnPoints` (`|MakeArray` (`SceneComponent.GetRelativeTransform` (`self.SpawnPoint_01`)) (`SceneComponent.GetRelativeTransform` (`self.SpawnPoint_02`)) (`SceneComponent.GetRelativeTransform` (`self.SpawnPoint_03`)))))

(fn `spawnBlocker`
  (bind _spawnpoints (`self.SpawnPoints`))
  (bind _asendless_run_character (cast `/Game/Blueprints/EndlessRunCharacter` (`GameplayStatics.GetPlayerCharacter` 0)))
  (if (> (`/Game/Blueprints/EndlessRunCharacter.totalCoins` _asendless_run_character) 10000)
    (`AddComponent|NODE_AddChildActorComponent-0` :`RelativeTransform` (`|GetArrayItem` _spawnpoints (`KismetMathLibrary.RandomIntegerInRange` 0 (`KismetArrayLibrary.Array_LastIndex` _spawnpoints))))))

(fn `spawnCoins`
  (bind _coinarea (`self.coinArea`))
  (bind _returnvalue_location (`KismetMathLibrary.BreakTransform` (`SceneComponent.GetRelativeTransform` _coinarea)))
  (bind _returnvalue (`KismetMathLibrary.Conv_VectorToTransform` (`KismetMathLibrary.RandomPointInBoundingBox` _returnvalue_location (`.BoxExtent` (`KismetSystemLibrary.GetComponentBounds` _coinarea)))))
  (for _ (range (+ (`KismetMathLibrary.RandomIntegerInRange` 3 10) 1))
    (switch `int` (`KismetMathLibrary.RandomIntegerInRange` 0 3)
      (:`Default`
        (`AddComponent|NODE_AddChildActorComponent-5` :`RelativeTransform` _returnvalue :!label _label))
      (:`0`
        (goto _label))
      (:`1`
        (`AddComponent|NODE_AddChildActorComponent-6` :`RelativeTransform` _returnvalue))
      (:`2`
        (`AddComponent|NODE_AddChildActorComponent-7` :`RelativeTransform` _returnvalue))
      (:`3`
        (`AddComponent|NODE_AddChildActorComponent-8` :`RelativeTransform` _returnvalue)))))

(fn `UserConstructionScript`
  (`self.setSpawnPoints`)
  (`self.spawnCoins`)
  (`self.spawnBlocker`))