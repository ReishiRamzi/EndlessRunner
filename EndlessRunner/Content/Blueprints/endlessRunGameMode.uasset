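; Game mode for an endless runner that creates the HUD and builds the opening stretch of track on BeginPlay.
; AddFloorTile spawns a random straight tile class at NextSpawnPoint, then advances that point to the new tile's attach transform to chain pieces end to end.
; A straight counter hands off to AddFloorTurn after a run of straights, which chains a random turn piece the same way and resets the count.
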(event `self.ReceiveBeginPlay`
  (bind _returnvalue (`|CreateWidget` "/Game/Blueprints/endlessRunHUD.endlessRunHUD_C"))
  (`UserWidget.AddToViewport` _returnvalue 0)
  (for _ (range 10)
    (`self.addFloorTile`)))

(fn `addFloorTile`
  (bind _floortilestype (`self.floorTilesType`))
  (if (> (`self.currentStraights`) 7)
    (`self.addFloorTurn`)
    (else
      (bind _returnvalue (`|SpawnActorFromClass` (`|GetArrayItem` _floortilestype (`KismetMathLibrary.RandomIntegerInRange` 0 (`KismetArrayLibrary.Array_LastIndex` _floortilestype))) (`self.nextSpawnPoint`) "Undefined" "OverrideRootScale" null null))
      (bind _asbp_floor_tile (cast `/Game/Blueprints/Tiles/BP_FloorTile` _returnvalue))
      (bind _attachpointtransform (`/Game/Blueprints/Tiles/BP_FloorTile.getAttachTransform` _asbp_floor_tile))
      (set `self.nextSpawnPoint` _attachpointtransform)
      (set `self.currentStraights` (+ (`self.currentStraights`) 1)))))

(fn `addFloorTurn`
  (bind _floorturns (`self.floorTurns`))
  (bind _returnvalue (`|SpawnActorFromClass` (`|GetArrayItem` _floorturns (`KismetMathLibrary.RandomIntegerInRange` 0 (`KismetArrayLibrary.Array_LastIndex` _floorturns))) (`self.nextSpawnPoint`) "Undefined" "OverrideRootScale" null null))
  (bind _asbp_floor_tile (cast `/Game/Blueprints/Tiles/BP_FloorTile` _returnvalue))
  (bind _attachpointtransform (`/Game/Blueprints/Tiles/BP_FloorTile.getAttachTransform` _asbp_floor_tile))
  (set `self.nextSpawnPoint` _attachpointtransform)
  (set `self.currentStraights` 0))

(fn `UserConstructionScript`)